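; Enemy drone actor that patrols between two points while periodically spawning Enemy_Drone_Bullet actors.
; BeginPlay caches two component world positions, and Tick moves toward the current one at constant speed via VInterpToConstant, with GetNextLocation cycling the index on arrival.
; A Delay on Tick throttles spawning at BombLocation to roughly every two seconds.
; Disconnected nodes hold unused movement variants, including a lerp with timed waypoint switching.
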(event `self.ReceiveBeginPlay`
  (bind _locationlist (`self.LocationList`))
  (`KismetArrayLibrary.Array_Add` _locationlist (`SceneComponent.K2_GetComponentLocation` (`self.Location1`)))
  (`KismetArrayLibrary.Array_Add` _locationlist (`SceneComponent.K2_GetComponentLocation` (`self.Location2`))))

(event `self.ReceiveTick`
  (params (DeltaSeconds :type "Float (single-precision)"))
  (bind _returnvalue (`self.K2_GetActorLocation`))
  (bind _bomblocation (`self.BombLocation`))
  (bind _output (`|GetArrayItem` (`self.LocationList`) (`self.Counter`)))
  (`|ExecutionSequence`
    (:`then_0`
      (`self.GetNextLocation` _returnvalue _output)
      (`self.K2_SetActorLocation` (`KismetMathLibrary.VInterpTo_Constant` _returnvalue _output DeltaSeconds 250.0)))
    (:`then_1`
      (`KismetSystemLibrary.Delay` 2.0)
      (`|SpawnActorFromClass` "/Game/MSA/Blueprints/Enemy_Drone_Bullet.Enemy_Drone_Bullet_C" (`KismetMathLibrary.MakeTransform` (`SceneComponent.K2_GetComponentLocation` _bomblocation) (`SceneComponent.K2_GetComponentRotation` _bomblocation)) "Undefined" "OverrideRootScale" null null))))

(fn `GetNextLocation`
  (params (A :type "Vector Structure") (B :type "Vector Structure"))
  (if (< (`KismetMathLibrary.Vector_Distance` A B) 0.1)
    (bind _result (`/Engine/EditorBlueprintResources/StandardMacros.IncrementInt` (`self.Counter`))
      (:`  `
        (if (>= _result (`KismetArrayLibrary.Array_Length` (`self.LocationList`)))
          (set `self.Counter` 0))))))

(fn `UserConstructionScript`)