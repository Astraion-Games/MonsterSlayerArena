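; Gameplay manager, apparently a GameMode, that populates the level with BP_EnemyBase monsters.
; On BeginPlay it caches the player as BP_Slayer and, if that cast succeeds, spawns the first monster.
; Tick spawns another whenever MonsterList holds fewer than three entries.
; Each monster appears at a random point in a square around the world origin and joins MonsterList, which this graph never prunes.
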(event `self.ReceiveBeginPlay`
  (bind _asbp_slayer (cast `/Game/MSA/Blueprints/BP_Slayer` (`GameplayStatics.GetPlayerPawn` 0)))
  (set `self.Char_Player` _asbp_slayer)
  (`self.SpawnMonster`))

(event `SpawnMonster`
  (bind _spawntransform (`self.MonsterSpawnLocation`))
  (bind _returnvalue (`|SpawnActorFromClass` "/Game/MSA/Blueprints/BP_EnemyBase.BP_EnemyBase_C" _spawntransform "Undefined" "OverrideRootScale" null null))
  (`KismetArrayLibrary.Array_Add` (`self.MonsterList`) _returnvalue))

(event `self.ReceiveTick`
  (params (DeltaSeconds :type "Float (single-precision)"))
  (if (< (`KismetArrayLibrary.Array_Length` (`self.MonsterList`)) 3)
    (`self.SpawnMonster`)))

(fn `MonsterSpawnLocation`
  (returns (SpawnTransform :type "Transform Structure"))
  (return (`KismetMathLibrary.MakeTransform` (`KismetMathLibrary.MakeVector` (`KismetMathLibrary.RandomFloatInRange` -350.0 350.0) (`KismetMathLibrary.RandomFloatInRange` -350.0 350.0) 100.0))))

(fn `UserConstructionScript`)